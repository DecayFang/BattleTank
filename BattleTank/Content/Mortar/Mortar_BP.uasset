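; Mortar Blueprint that assembles a mortar from body, dome and barrel meshes and hooks it up for aiming.
; The construction script assigns the static mesh for each of the three parts.
; On BeginPlay it initializes the MortarAiming component, passing the barrel as barrel and the dome as turret, leaving the aiming logic to that component.
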(event `self.ReceiveBeginPlay`
  (`TankAimingComponent.Initialize` (`self.MortarAiming`) (`self.MortarBarrel`) (`self.MortarDome`)))

(fn `UserConstructionScript`
  (`StaticMeshComponent.SetStaticMesh` (`self.MortarBody`) "/Game/Mortar/mortar_body.mortar_body")
  (`StaticMeshComponent.SetStaticMesh` (`self.MortarDome`) "/Game/Mortar/mortar_dome.mortar_dome")
  (`StaticMeshComponent.SetStaticMesh` (`self.MortarBarrel`) "/Game/Mortar/mortar_barrel.mortar_barrel"))