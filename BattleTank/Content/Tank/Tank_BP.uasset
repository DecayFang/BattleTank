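; Player-drivable tank Blueprint with mouse-look aiming, firing, switchable first/third-person cameras and a health bar widget linked to the tank.
; Input rotates an azimuth gimbal and elevation arm, fires through AimingComponent, and drives MovementComponent fly-by-wire, leaving direct track throttle unwired.
; BeginPlay hands barrel, turret and tracks to those components.
; The construction script assigns meshes, projectile class, and track physical material and hit events.
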(event `self.ReceiveBeginPlay`
  (`ActorComponent.Activate` (`self.ThridPerson`) false)
  (`ActorComponent.Deactivate` (`self.FirstPerson`))
  (`TankAimingComponent.Initialize` (`self.AimingComponent`) (`self.Barrel`) (`self.Turret`))
  (`TankMovementComponent.Initialize` (`self.MovementComponent`) (`self.LeftTrack`) (`self.RightTrack`))
  (`self.InitializeHealthBarWidget`))

(event `InputAxis|AimAzimuth`
  (params (AxisValue :type "Float (single-precision)"))
  ;[1 1 1] Aim Input Bindings
  (`SceneComponent.K2_AddLocalRotation` (`self.AzimuthGimbal`) (`KismetMathLibrary.MakeRotator` 0.0 0.0 (* AxisValue (`self.MouseSensitivity`) (`GameplayStatics.GetWorldDeltaSeconds`))) false false))

(event `InputAxis|AimElevation`
  (params (AxisValue :type "Float (single-precision)"))
  ;[1 1 1] Aim Input Bindings
  (`SceneComponent.K2_AddLocalRotation` (`self.ElevationArm`) (`KismetMathLibrary.MakeRotator` 0.0 (* AxisValue (`self.MouseSensitivity`) (`GameplayStatics.GetWorldDeltaSeconds`))) false false))

(event `InputAction|SwapCamera`
  (params (Key :type "Key Structure"))
  ;[1 1 1] Camera Switching
  (:`Released`
    (`ActorComponent.ToggleActive` (`self.FirstPerson`))
    (`ActorComponent.ToggleActive` (`self.ThridPerson`))))

(event `InputAction|TankFire`
  (params (Key :type "Key Structure"))
  ;[1 1 1] Aim Input Bindings
  (:`Pressed`
    (`TankAimingComponent.Fire` (`self.AimingComponent`))))

(event `InputAxis|LeftThrottle`
  (params (AxisValue :type "Float (single-precision)"))
  ;[1 1 1] Movement Input Bindings
  ;;[1 1 1] Connect the exec nodes if you want manual control
)

(event `InputAxis|RightThrottle`
  (params (AxisValue :type "Float (single-precision)"))
  ;[1 1 1] Movement Input Bindings
  ;;[1 1 1] Connect the exec nodes if you want manual control
)

(event `InputAxis|MoveForward`
  (params (AxisValue :type "Float (single-precision)"))
  ;[1 1 1] Movement Input Bindings
  ;;[1 1 1] Fly-by-Wire control
  (`TankMovementComponent.IntendMoveForward` (`self.MovementComponent`) AxisValue))

(event `InputAxis|TurnClockwise`
  (params (AxisValue :type "Float (single-precision)"))
  ;[1 1 1] Movement Input Bindings
  ;;[1 1 1] Fly-by-Wire control
  (`TankMovementComponent.IntendTurnClockwise` (`self.MovementComponent`) AxisValue))

(fn `InitializeHealthBarWidget`
  (bind _ashealth_bar_bp (cast `/Game/UI/HealthBar_BP` (`WidgetComponent.GetWidget` (`self.HealthBarContainer`)))
    (:`then`
      (set `/Game/UI/HealthBar_BP.AttachedTank` self _ashealth_bar_bp))
    (:`CastFailed`
      (`KismetSystemLibrary.PrintString` "Error: Failed to cast Widget to HealthBar_BP"))))

(fn `UserConstructionScript`
  (`StaticMeshComponent.SetStaticMesh` (`self.Turret`) "/Game/Tank/tank_fbx_Turret.tank_fbx_Turret")
  (`StaticMeshComponent.SetStaticMesh` (`self.Barrel`) "/Game/Tank/tank_fbx_Barrel.tank_fbx_Barrel")
  (`StaticMeshComponent.SetStaticMesh` (`self.LeftTrack`) "/Game/Tank/tank_fbx_Track.tank_fbx_Track")
  (`StaticMeshComponent.SetStaticMesh` (`self.RightTrack`) "/Game/Tank/tank_fbx_Track.tank_fbx_Track")
  (`PrimitiveComponent.SetPhysMaterialOverride` (`self.LeftTrack`) "/Game/Tank/TrackPhyMat.TrackPhyMat")
  (`PrimitiveComponent.SetPhysMaterialOverride` (`self.RightTrack`) "/Game/Tank/TrackPhyMat.TrackPhyMat")
  (set `TankAimingComponent.ProjectileBlueprint` "/Game/Projectile/Projectile_BP.Projectile_BP_C" (`self.AimingComponent`))
  (`PrimitiveComponent.SetNotifyRigidBodyCollision` (`self.LeftTrack`) true) ; NotifyRigidBodyCollision (both in c++ and BP) = \nSimulation Generates Hit Events in Collision setting
  (`PrimitiveComponent.SetNotifyRigidBodyCollision` (`self.RightTrack`) true))